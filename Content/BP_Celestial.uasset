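; BP_Celestial is a celestial body actor that repositions itself relative to a Parent, apparently for orbital motion.
; Each Tick, while Parent is valid, it takes the offset from Parent to its Planet component and rotates it in yaw by Rotation.
; That vector becomes the actor's world location without sweep; Parent's location is not added back, and Rotation is not changed in these graphs.
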(event `self.ReceiveTick`
  (params (DeltaSeconds :type "Float (single-precision)"))
  ;[1 1 1] Check if has valid parent
  (if (`KismetSystemLibrary.IsValid` (`self.Parent`))
    (`self.K2_SetActorLocation` (`KismetMathLibrary.GreaterGreater_VectorRotator` (- (`SceneComponent.K2_GetComponentLocation` (`self.Planet`)) (`self.K2_GetActorLocation` (`self.Parent`))) (`KismetMathLibrary.MakeRot` 0.0 (`self.Rotation`))))))

(fn `UserConstructionScript`)